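; Player character with side-on movement, limited multi-jumps, mid-air spinning and respawning.
; Jumps launch on release along a rotation-derived vector; hold time only accumulates airborne, and SetJumpPower raises it to at least the maximum.
; Tick rolls the airborne body by horizontal speed and faces it left or right when grounded; hits restore jumps.
; BeginPlay spawns a follow camera and saves the spawn location, where death (debug key R) spawns a replacement.
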(event Custom|DeathEvent_Event
  (Development|PrintString "should reset")
  (Game|SpawnActorfromClass "PlayerBP_C" (Math|Conversions|ToTransform(Vector) (Variables|Default|GetlastSafeRespawnLocation)) "Undefined" "MultiplyWithRoot" 0 0)
  (Actor|DestroyActor))

(event Input|EnhancedActionEvents|EnhancedInputActionIA_Jump
  (params (ActionValue :type Boolean) (ElapsedSeconds :type Float%20%28double-precision%29) (TriggeredSeconds :type Float%20%28double-precision%29) (InputAction :type Input%20Action%20Object%20Reference :default "/Game/ThirdPerson/Input/Actions/IA_Jump.IA_Jump"))
  (:Started
    (if (> (Variables|Default|GetjumpsAvailable) 0)
      (Variables|Default|SetholdsJump true)
      (Variables|Default|SetjumpsAvailable (- (Variables|Default|GetjumpsAvailable) 1))))
  (:Completed
    (if (Variables|Default|GetholdsJump)
      (Variables|Default|SetholdsJump false)
      (CallFunction|SetJumpPower)
      (CallFunction|ExecuteJump)
      (Variables|Default|SetisOnFloor false)
      (Variables|Default|SetjumpHoldTime 0.0)
      (Utilities|FlowControl|DoOnce false) ; enters at Reset
    )))

(event Input|EnhancedActionEvents|EnhancedInputActionIA_Move
  (params (ActionValue :type Vector%202D%20Structure) (ElapsedSeconds :type Float%20%28double-precision%29) (TriggeredSeconds :type Float%20%28double-precision%29) (InputAction :type Input%20Action%20Object%20Reference :default "/Game/ThirdPerson/Input/Actions/IA_Move.IA_Move"))
  (bind _returnvalue (Pawn|GetControlRotation :!class /Script/Engine.Pawn))
  (Pawn|Input|AddMovementInput (Math|Vector|GetRightVector (Math|Rotator|MakeRotator (.roll _returnvalue) (.pitch _returnvalue) (.yaw _returnvalue))) (.x ActionValue) false)
  (if (Variables|Default|GetisOnFloor)
    (if (> (.y (Transformation|GetVelocity)) 0.0)
      (Variables|Default|SetlastDirectionRight true)
      (else
        (Variables|Default|SetlastDirectionRight false)))))

(event EventBeginPlay
  (Development|PrintString "spawned")
  (bind _asplayer_controller (Utilities|Casting|CastToPlayerController (Pawn|GetController)))
  (Utilities|IsValid (PlayerController|LocalPlayerSubsystems|GetEnhancedInputLocalPlayerSubsystem _asplayer_controller)
    (:Is%20Valid
      (Input|AddMappingContext (PlayerController|LocalPlayerSubsystems|GetEnhancedInputLocalPlayerSubsystem _asplayer_controller) "/Game/ThirdPerson/Input/IMC_Default.IMC_Default" 0 "(bIgnoreAllPressedKeysUntilRelease=True,bForceImmediately=False,bNotifyUserSettings=False)")
      (Variables|Default|SetlastSafeRespawnLocation (Transformation|GetActorLocation))
      ;[0.05098 0.05098 0.05098] Follow Camera mapping
      (bind _returnvalue (Game|SpawnActorfromClass "/Game/ThirdPerson/Blueprints/BP_Camera-Lacho.BP_Camera-Lacho_C" (Math|Transform|MakeTransform (Transformation|GetActorLocation) "0, 0, 0" "1.000000,1.000000,1.000000") "Undefined" "MultiplyWithRoot" 0 self 0))
      (Game|Player|SetViewTargetwithBlend (Game|GetPlayerController 0) _returnvalue 0.0 "VTBlend_Linear" 0.0 false))))

(event EventTick
  (params (DeltaSeconds :type Float%20%28single-precision%29))
  (Variables|Default|SetcurrentDeltaSeconds DeltaSeconds)
  (CallFunction|RotateCharacterMidAir)
  (if true
    (if (Variables|Default|GetisOnFloor)
      (CallFunction|RotateCharacteronGround)
      (elif (Variables|Default|GetholdsJump)
        (Variables|Default|SetjumpHoldTime (+ (Variables|Default|GetjumpHoldTime) (Variables|Default|GetcurrentDeltaSeconds)))))))

(event Collision|EventHit
  (params (MyComp :type Primitive%20Component%20Object%20Reference) (Other :type Actor%20Object%20Reference) (OtherComp :type Primitive%20Component%20Object%20Reference) (bSelfMoved :type Boolean) (HitLocation :type Vector :default "0, 0, 0") (HitNormal :type Vector :default "0, 0, 0") (NormalImpulse :type Vector :default "0, 0, 0") (Hit :type Hit%20Result%20Structure%20%28by%20ref%29))
  (Utilities|FlowControl|DoOnce false
    (:Completed
      (Variables|Default|SetisOnFloor true)
      (Variables|Default|SetjumpsAvailable (Variables|Default|GetmaxJumps)))))

(event Input|KeyboardEvents|DebugKeyR
  (params (Key :type Key%20Structure :default "None") (ActionValue :type Input%20Action%20Value%20Structure))
  (:Pressed
    (Development|PrintString "Hard reset")
    (Default|CallDeathEvent)))

(fn ConstructionScript)

(fn ExecuteJump
  (bind _returnvalue (Transformation|GetActorRotation))
  (Character|LaunchCharacter (Math|Rotator|GetRotationXVector (Math|Transform|TransformRotation (Math|Transform|MakeTransform "0, 0, 0" (* _returnvalue (* (Variables|Default|GetjumpHoldTime) 3e+03))) _returnvalue)) false false))

(fn SetJumpPower
  (if (not (> (Variables|Default|GetjumpHoldTime) (Variables|Default|GetmaxJumpHoldTime)))
    (Variables|Default|SetjumpHoldTime (Variables|Default|GetmaxJumpHoldTime))))

(fn RotateCharacterMidAir
  (if (Variables|Default|GetisOnFloor)
    (Class|Actor|AddActorWorldRotation (Math|Rotator|MakeRotator (.roll (Math|Conversions|RotationFromXVector (Math|Interpolation|VInterpTo (Math|Vector|MakeVector (.roll (Transformation|GetActorRotation)) 0.0 0.0) "0, 0, 0" (Variables|Default|GetcurrentDeltaSeconds) 3.0))) 0.0 0.0))
    (Variables|Default|SetcurrentRotation 1.0)
    (else
      (bind _output_get (Variables|Default|SetcurrentRotation (+ (* (Variables|Default|GetcurrentDeltaSeconds) (Math|Float|MapRangeClamped (Math|Float|Absolute(Float) (.y (Transformation|GetVelocity))) 0.0 6e+02 0.0 4e+02)) (Variables|Default|GetcurrentRotation))))
      (Class|Actor|AddActorWorldRotation (Math|Rotator|MakeRotator _output_get 0.0 0.0)))))

(fn RotateCharacteronGround
  (bind _returnvalue (Transformation|GetActorRotation))
  (bind _returnvalue_2 (Transformation|GetActorRotation))
  (if (Variables|Default|GetlastDirectionRight)
    (Transformation|SetActorRotation (Math|Rotator|MakeRotator (.roll _returnvalue_2) (.pitch _returnvalue_2) 9e+01))
    (else
      (Transformation|SetActorRotation (Math|Rotator|MakeRotator (.roll _returnvalue) (.pitch _returnvalue) -9e+01)))))